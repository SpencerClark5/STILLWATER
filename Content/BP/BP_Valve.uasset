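; BP_Valve is an interactable pipe valve that raises and lowers two water bodies when the player turns it.
; Interaction alternately plays and reverses the Rot timeline, which yaws the handle and lerps each water actor's height between its top and bottom values on separate tracks.
; CanTurn blocks input and hides the HUD prompt during a turn, while an audio emitter plays until the timeline finishes.
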(event `self.ReceiveBeginPlay`
  (`parent.ReceiveBeginPlay`)
  (`TimelineComponent.SetPlayRate` (`self.Rot`) (`self.Play Rate`))
  (set `/Game/Developers/JTLib/Audio/BP_AudioEmitterComponent.AttachedSoundLocation` (`self.Object Mesh`) (`self.AudioEmitterComponent`)))

(event `/Game/BP/Interfaces/I_Interactable.Show Info`
  (params (HUD :type "/Game/BP/Widgets/WBP_HUD Object Reference"))
  (if (`self.CanTurn?`)
    (`/Game/BP/Widgets/WBP_HUD.Set Info Text` HUD "Press [E] to turn valve")))

(event `/Game/BP/Interfaces/I_Object.Interact object`
  (bind _water_1 (`self.Water_1`))
  (bind _water_2 (`self.Water_2`))
  (bind (_returnvalue_x _returnvalue_y) (`KismetMathLibrary.BreakVector` (`self.K2_GetActorLocation` _water_2)))
  (bind (_returnvalue_x_2 _returnvalue_y_2) (`KismetMathLibrary.BreakVector` (`self.K2_GetActorLocation` _water_1)))
  (if (`self.CanTurn?`)
    (set `self.CanTurn?` false)
    (`/Game/Developers/JTLib/Audio/BP_AudioEmitterComponent.TogglePlaying` (`self.AudioEmitterComponent`) true)
    (`/Engine/EditorBlueprintResources/StandardMacros.FlipFlop`
      (:`A`
        (bind (_direction _rot _water_1_2 _water_2_2) (`Timeline|Rot` :!via `PlayFromStart` :!label _label)
          (:`Update`
            ;[1 1 1] Rot valve handle
            (`SceneComponent.K2_SetRelativeRotation` (`self.Pipe_Valve_Handle`) (`KismetMathLibrary.MakeRotator` 0.0 0.0 _rot) false false)
            ;[1 1 1] Set height of water 1
            (`self.K2_SetActorLocation` _water_1 (`KismetMathLibrary.MakeVector` _returnvalue_x_2 _returnvalue_y_2 (`KismetMathLibrary.Lerp` (`self.Top_Height_1`) (`self.Bottom_Height_1`) _water_1_2)) false false)
            ;[1 1 1] Set height of water 2
            (`self.K2_SetActorLocation` _water_2 (`KismetMathLibrary.MakeVector` _returnvalue_x _returnvalue_y (`KismetMathLibrary.Lerp` (`self.Top_Height_2`) (`self.Bottom_Height_2`) _water_2_2)) false false))
          (:`Finished`
            (set `self.CanTurn?` true)
            (`/Game/Developers/JTLib/Audio/BP_AudioEmitterComponent.TogglePlaying` (`self.AudioEmitterComponent`) false))))
      (:`B`
        (goto _label :!via `ReverseFromEnd`)))))

(fn `UserConstructionScript`
  (`parent.UserConstructionScript`))