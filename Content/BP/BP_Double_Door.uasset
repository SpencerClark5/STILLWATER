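; Interactable double door that opens, closes and can start locked, based on an editor-set Status enum.
; Interacting while unlocked plays a sound through the player's audio component and plays or reverses a Timeline that rotates both door meshes.
; ShowInfo sets HUD prompts for the current state when the player looks at the door.
; Unlock switches it to closed and interactable.
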(event `self.ReceiveBeginPlay`
  ;[1 1 1] Grabs whatever the editor has set to and sets status
  (switch `/Game/Enums/EN_DoorStatus` (`self.Status`)
    (:`NewEnumerator2`
      (set `self.IsLocked` true))
    (:`NewEnumerator0`
      (set `self.IsLocked` false :!label _label))
    (:`NewEnumerator1`
      (goto _label)))
  (bind _returnvalue (`GameplayStatics.GetActorOfClass` "/Game/FirstPerson/Blueprints/BP_FirstPersonCharacter_New.BP_FirstPersonCharacter_New_C"))
  (set `self.Character BP` _returnvalue))

(event `self.Interact object`
  ;[1 1 1] Change the status of the door enum, change the rotation of the door
  (if (not (`self.IsLocked`))
    (`/Game/Developers/JTLib/Audio/BP_PlayerAudioComponent.PlaySoundAttached` (`self.GetComponentByClass` (`self.Character BP`) "/Game/Developers/JTLib/Audio/BP_PlayerAudioComponent.BP_PlayerAudioComponent_C") (`|MakeArray` "/Game/Audio/ObjectSounds/DoorOpen_2.DoorOpen_2" :!type "SoundWave Object Reference") (`self.SoundLocation`))
    (switch `/Game/Enums/EN_DoorStatus` (`self.Status`)
      (:`NewEnumerator0`
        (set `self.Status` "NewEnumerator1")
        ;[1 1 1] With a duration of 0.5 seconds, lerp from 0 degrees of Z rotation to 90
        (bind (_direction _door_z_rotation _newtrack_0) (`Timeline|Timeline` :!label _label_2)
          (:`Update`
            ;[1 1 1] Based on the current lerp value, set the rotation
            (`SceneComponent.K2_SetRelativeRotation` (`self.Object Mesh`) (`KismetMathLibrary.MakeRotator` 0.0 0.0 _door_z_rotation) false false)
            (`SceneComponent.K2_SetRelativeRotation` (`self.IndustrialDoor_Door1`) (`KismetMathLibrary.MakeRotator` 0.0 0.0 _newtrack_0) false false))))
      (:`NewEnumerator1`
        (set `self.Status` "NewEnumerator0")
        (goto _label_2 :!via `Reverse`)))))

(event `/Game/BP/Classes/InteractableBaseClass.Show Info`
  (params (HUD :type "/Game/BP/Widgets/WBP_HUD Object Reference"))
  ;[1 1 1] When the players normal looking raycast hits the door, display some text on the widget
  (switch `/Game/Enums/EN_DoorStatus` (`self.Status`)
    (:`NewEnumerator2`
      (`/Game/BP/Widgets/WBP_HUD.Set Info Text` HUD "Door is locked")
      (set `TextBlock.Text` "Use LMB to unlock door" (`/Game/BP/Widgets/WBP_HUD.InteractInfo` HUD)))
    (:`NewEnumerator0`
      (`/Game/BP/Widgets/WBP_HUD.Set Info Text` HUD "Press [E] to open door"))
    (:`NewEnumerator1`
      (`/Game/BP/Widgets/WBP_HUD.Set Info Text` HUD "Press [E] to close door"))))

(event `/Game/BP/Interfaces/I_Unlock.Unlock`
  (set `self.Status` "NewEnumerator0")
  (set `self.IsLocked` false))

(fn `UserConstructionScript`)