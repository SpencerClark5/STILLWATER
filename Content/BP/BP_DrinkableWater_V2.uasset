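; Drinkable water body that temporarily reveals hidden actors and can be raised or lowered.
; Drinking adds M_DrankWater to the "Switch"-tagged post-process volume and shows I_Visible and I_KeyVisible actors, reverting after a delay but leaving held keys visible.
; Raise, Lower and LevelToggle drive a timeline that moves the water and toggles a blocking collider for deep water.
; Hitting that blocker plays a subtitle on the player, gated against repeats.
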(event `self.ReceiveBeginPlay`
  (`|ExecutionSequence`
    (:`then_0`
      (`TimelineComponent.SetPlayRate` (`self.Water Level`) (`self.Play Rate`)))
    (:`then_1`
      (if (not (`self.WaterToDeep?`))
        (`PrimitiveComponent.SetCollisionEnabled` (`self.Water Block`) "NoCollision")))
    (:`then_2`
      ;[1 0.1958 0.9119] Set post process to variable in order to allow shader to be added later (during runtime)
      (bind _outactors (`GameplayStatics.GetAllActorsOfClassWithTag` "/Script/Engine.PostProcessVolume" "Switch"))
      (for _array_element _outactors
        (set `self.PostProcess` _array_element)
        (bind _outactors_2 (`GameplayStatics.GetAllActorsOfClass` "/Game/BP/Items/BP_Key_Howie.BP_Key_Howie_C"))
        (`self.SetActorHiddenInGame` _outactors_2 true)
        (`self.SetActorEnableCollision` _outactors_2 false)))))

(event `self.Interact object`
  (bind _weightedblendable (make `WeightedBlendable` 1.0 "/Game/Materials/Shaders/M_DrankWater.M_DrankWater"))
  (bind _array (break `WeightedBlendables` (`.WeightedBlendables` (break `PostProcessSettings` (`PostProcessVolume.Settings` (`self.PostProcess`))))))
  ;[1 0.08653 0.7857] Add shader to post-processing volume when water is drank
  (`KismetSystemLibrary.Delay` 0.2)
  (`KismetArrayLibrary.Array_Add` _array _weightedblendable)
  (set `self.WaterIsDrank` true)
  (bind _outactors (`GameplayStatics.GetAllActorsWithInterface` "/Game/BP/Interfaces/I_Visible.I_Visible_C"))
  (for _array_element _outactors
    (message `/Game/BP/Interfaces/I_Visible.Toggle Visibility` _array_element)
    (`self.SetActorHiddenInGame` _array_element false)
    (`self.SetActorEnableCollision` _array_element true)
    (bind _outactors_2 (`GameplayStatics.GetAllActorsWithInterface` "/Game/BP/Interfaces/I_KeyVisible.I_KeyVisible_C"))
    (for _array_element_2 _outactors_2
      (`self.SetActorHiddenInGame` _array_element_2 false)
      (`self.SetActorEnableCollision` _array_element_2 true)
      (`KismetSystemLibrary.Delay` 30.0)
      (`KismetArrayLibrary.Array_RemoveItem` _array _weightedblendable)
      (set `self.WaterIsDrank` false)
      (for _array_element_3 _outactors
        (`self.SetActorHiddenInGame` _array_element_3 true)
        (`self.SetActorEnableCollision` _array_element_3 false)
        (for _array_element_4 _outactors_2
          (bind _asitem_base_class (cast `/Game/BP/Classes/ItemBaseClass` _array_element_4))
          (if (not (`/Game/BP/Classes/ItemBaseClass.isHeld` _asitem_base_class))
            (`self.SetActorHiddenInGame` _array_element_4 true)
            (`self.SetActorEnableCollision` _array_element_4 false)))))))

(event `self.Show Info`
  (params (HUD :type "/Game/BP/Widgets/WBP_HUD Object Reference"))
  ;[0.2033 0.6384 1] Display text for water
  (`/Game/BP/Widgets/WBP_HUD.Set Info Text` HUD "Press [E] to drink"))

(event `/Game/BP/Interfaces/I_WaterLevel.Raise`
  (bind _water_block (`self.Water Block`))
  (bind (_returnvalue_x _returnvalue_y) (`KismetMathLibrary.BreakVector` (`SceneComponent.K2_GetComponentLocation` (`self.DefaultSceneRoot`))))
  ;[1 1 1] Water Raise/Lower
  (set `self.WaterToDeep?` true :!label _label)
  (`PrimitiveComponent.SetCollisionEnabled` _water_block "QueryAndPhysics")
  (bind (_direction _lerp) (`Timeline|Water Level` :!via `PlayFromStart` :!label _label_2)
    (:`Update`
      (`self.K2_SetActorLocation` (`KismetMathLibrary.MakeVector` _returnvalue_x _returnvalue_y (`KismetMathLibrary.Lerp` (`self.Water Height Top`) (`self.Water Height Bottom`) _lerp))))
    (:`Finished`
      (if (not (`self.WaterToDeep?`))
        (`PrimitiveComponent.SetCollisionEnabled` _water_block "NoCollision")))))

(event `/Game/BP/Interfaces/I_WaterLevel.LevelToggle`
  ;[1 1 1] Water Raise/Lower
  (if (`self.WaterToDeep?`)
    (set `self.WaterToDeep?` false :!label _label_3)
    (goto _label_2 :!via `ReverseFromEnd`)
    (else
      (goto _label))))

(event `/Game/BP/Interfaces/I_WaterLevel.Lower`
  ;[1 1 1] Water Raise/Lower
  (goto _label_3))

(event `self.Water Block.OnComponentHit`
  (params (HitComponent :type "PrimitiveComponent Object Reference") (OtherActor :type "Actor Object Reference") (OtherComp :type "PrimitiveComponent Object Reference") (NormalImpulse :type "Vector Structure") (Hit :type "HitResult Structure (by ref)"))
  (bind _dialogue (`self.Dialogue`))
  (bind _update_time (`self.Update Time`))
  ;[1 1 1] Dialog to say water is to deep
  (bind _asbp_first_person_character_new (cast `/Game/FirstPerson/Blueprints/BP_FirstPersonCharacter_New` OtherActor))
  (if (`self.Finished`)
    (set `self.Finished` false)
    (`/Game/Developers/JTLib/WBP_SUBTITLE.MakeSubtitle` (`/Game/FirstPerson/Blueprints/BP_FirstPersonCharacter_New.Subtitle Widget` _asbp_first_person_character_new) _dialogue _update_time (`self.End Delay`))
    (`KismetSystemLibrary.Delay` (+ (* (`KismetStringLibrary.Len` _dialogue) _update_time) (`self.Hang TIme`)))
    (set `self.Finished` true)))

(fn `UserConstructionScript`)