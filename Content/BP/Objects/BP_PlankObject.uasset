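; BP_PlankObject is a plank placement spot that starts invisible and non-blocking to pawns and physics bodies.
; A repeating delay loop shows a highlight overlay when the player holds a BP_PlankItem within range.
; ShowInfo sets the HUD placement prompt while a plank is held.
; Turnonplank, guarded to run once by the Deactivated flag, applies the overlay and restores blocking collision.
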(event `self.ReceiveBeginPlay`
  (bind _object_mesh (`self.Object Mesh`))
  ;[1 1 1] Sets the object to invis and disables collision
  (`PrimitiveComponent.SetCollisionResponseToChannel` _object_mesh "ECC_Pawn" "ECR_Ignore")
  (`PrimitiveComponent.SetCollisionResponseToChannel` _object_mesh "ECC_PhysicsBody" "ECR_Ignore")
  (`PrimitiveComponent.SetMaterial` (`self.Object Mesh`) 0 "/Game/Materials/M_Invisable.M_Invisable")
  (bind _returnvalue (`GameplayStatics.GetActorOfClass` "/Game/FirstPerson/Blueprints/BP_FirstPersonCharacter_New.BP_FirstPersonCharacter_New_C"))
  (set `self.Character BP_0` _returnvalue)
  (`self.LoopForHighlight`))

(event `Turn on plank`
  (bind _object_mesh (`self.Object Mesh`))
  ;[1 1 1] Change the status of the door enum, change the rotation of the door
  (if (not (`self.Deactivated`))
    (`MeshComponent.SetOverlayMaterial` (`self.Object Mesh`) "/Game/StarterContent/Props/Materials/M_TableRound.M_TableRound")
    (`KismetSystemLibrary.PrintString` "interacted")
    (set `self.Deactivated` true)
    (`PrimitiveComponent.SetCollisionResponseToChannel` _object_mesh "ECC_Pawn" "ECR_Block")
    (`PrimitiveComponent.SetCollisionResponseToChannel` _object_mesh "ECC_PhysicsBody" "ECR_Block")))

(event `/Game/BP/Classes/InteractableBaseClass.Show Info`
  (params (HUD :type "/Game/BP/Widgets/WBP_HUD Object Reference"))
  ;[1 1 1] If the player is holding a plank, display that they can put it here
  (cast `/Game/BP/Items/BP_PlankItem` (`/Game/FirstPerson/Blueprints/BP_FirstPersonCharacter_New.Held Item` (`self.Character BP_0`)))
  (`/Game/BP/Widgets/WBP_HUD.Set Info Interact` HUD "Press LMB to place plank"))

(event `LoopForHighlight`
  ;[1 1 1] If the player has a plank, display highlight at a certain distance
  (if (`/Game/FirstPerson/Blueprints/BP_FirstPersonCharacter_New.HasItem` (`self.Character BP_0`)) :!label _label
    (cast `/Game/BP/Items/BP_PlankItem` (`/Game/FirstPerson/Blueprints/BP_FirstPersonCharacter_New.Held Item` (`self.Character BP_0`))
      (:`then`
        (if (< (`self.GetDistanceTo` (`self.Character BP_0`)) 2000.0)
          (`MeshComponent.SetOverlayMaterial` (`self.Object Mesh`) "/Game/StarterContent/Props/Materials/M_TableRound.M_TableRound")
          (else
            (`MeshComponent.SetOverlayMaterial` (`self.Object Mesh`) "/Game/Materials/M_Invisable.M_Invisable")))
        (`KismetSystemLibrary.Delay` 0.1)
        (goto _label))
      (:`CastFailed`
        _)))
  (`KismetSystemLibrary.Delay` 0.1)
  (goto _label))

(fn `UserConstructionScript`)