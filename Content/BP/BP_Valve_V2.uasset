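; BP_Valve_V2 is an interactable valve that toggles the level of linked water actors and shows a HUD prompt while it can be turned.
; Each interaction starts valve audio and alternately plays or reverses a timeline that yaws the handle, stopping the audio when it finishes.
; It also calls LevelToggle through I_WaterLevel on WaterArray entries, locking interaction for the longest duration derived from their play rates.
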(event `self.ReceiveBeginPlay`
  (`parent.ReceiveBeginPlay`)
  (set `/Game/Developers/JTLib/Audio/BP_AudioEmitterComponent.AttachedSoundLocation` (`self.Object Mesh`) (`self.AudioEmitterComponent`)))

(event `self.ReceiveTick`
  (params (DeltaSeconds :type "Float (single-precision)"))
  (`parent.ReceiveTick` DeltaSeconds))

(event `/Game/BP/Classes/InteractableBaseClass.Show Info`
  (params (HUD :type "/Game/BP/Widgets/WBP_HUD Object Reference"))
  (if (`self.CanTurn?`)
    (`/Game/BP/Widgets/WBP_HUD.Set Info Text` HUD "Press [E] to turn valve")))

(event `self.Interact object`
  (if (`self.CanTurn?`)
    (set `self.CanTurn?` false)
    (`/Game/Developers/JTLib/Audio/BP_AudioEmitterComponent.TogglePlaying` (`self.AudioEmitterComponent`) true)
    (`|ExecutionSequence`
      (:`then_0`
        (`/Engine/EditorBlueprintResources/StandardMacros.FlipFlop`
          (:`A`
            (bind (_direction _rot) (`Timeline|Rot` :!via `PlayFromStart` :!label _label)
              (:`Update`
                (`SceneComponent.K2_SetRelativeRotation` (`self.Pipe_Valve_Handle`) (`KismetMathLibrary.MakeRotator` 0.0 0.0 _rot) false false))
              (:`Finished`
                (`/Game/Developers/JTLib/Audio/BP_AudioEmitterComponent.TogglePlaying` (`self.AudioEmitterComponent`) false))))
          (:`B`
            (goto _label :!via `ReverseFromEnd`))))
      (:`then_1`
        ;[1 1 1] Flipp water height and get the  longest time
        (for _array_element (`self.Water Array`)
          (bind _asi_water_level (cast `/Game/BP/Interfaces/I_WaterLevel` _array_element))
          (`/Game/BP/Interfaces/I_WaterLevel.LevelToggle` _asi_water_level)
          (bind _returnvalue (/ 5.0 (`/Game/BP/BP_DrinkableWater_V2.Play Rate` _array_element)))
          (if (> _returnvalue (`self.Delay`))
            (set `self.Delay` _returnvalue)))
        (`KismetSystemLibrary.Delay` (`self.Delay`))
        (set `self.CanTurn?` true)))))

(fn `UserConstructionScript`
  (`parent.UserConstructionScript`))