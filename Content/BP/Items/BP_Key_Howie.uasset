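; BP_Key_Howie is a carryable key item that unlocks its assigned Door and is consumed on use.
; Interacting raycasts from the character, unlocking that Door or showing a "Wrong Door" subtitle on other locked single or double doors.
; Dropping traces from the camera to place the key on the surface, falling back to floor traces in front of the player, and clears the anim blueprint's HasRifle flag.
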(event `self.DropItem`
  (bind _character_bp (`self.Character BP`))
  (bind _returnvalue (`self.K2_GetActorLocation` _character_bp))
  (bind _firstpersoncamera (`/Game/FirstPerson/Blueprints/BP_FirstPersonCharacter_New.FirstPersonCamera` (`self.Character BP`)))
  (bind _returnvalue_2 (`SceneComponent.K2_GetComponentLocation` _firstpersoncamera))
  ;[1 1 1] Set down on thing looking at
  (bind (_outhit _returnvalue_3) (`KismetSystemLibrary.LineTraceSingle` :`Start` _returnvalue_2 :`End` (+ _returnvalue_2 (* (`SceneComponent.GetForwardVector` _firstpersoncamera) 500.0)) :`TraceChannel` "TraceTypeQuery1" :`DrawDebugType` "ForDuration"))
  (if _returnvalue_3
    (`PrimitiveComponent.SetCollisionEnabled` (`self.Item mesh`) "QueryAndPhysics")
    (`self.K2_DetachFromActor` "KeepWorld" "KeepWorld" "KeepWorld")
    (bind (_bblockinghit _binitialoverlap _time _distance _location _impactpoint _normal) (`GameplayStatics.BreakHitResult` _outhit))
    (`self.K2_SetActorTransform` (`KismetMathLibrary.MakeTransform` _location (`KismetMathLibrary.Conv_VectorToRotator` (- _normal (0.0 -90.0 0.0)))))
    (bind _asfirst_person_anim_bp (cast `/Game/FirstPersonArms/Animations/FirstPerson_AnimBP` (`SkeletalMeshComponent.GetAnimInstance` (`/Game/FirstPerson/Blueprints/BP_FirstPersonCharacter_New.FirstPersonMesh` (`self.Character BP`)))))
    (set `/Game/FirstPersonArms/Animations/FirstPerson_AnimBP.HasRifle` false _asfirst_person_anim_bp)
    (else
      ;[1 1 1] If cant set on looking at set on floor infront
      (bind (_outhit_2 _returnvalue_4) (`KismetSystemLibrary.LineTraceSingle` :`Start` _returnvalue :`End` (- _returnvalue (0.0 0.0 300.0)) :`TraceChannel` "TraceTypeQuery1" :`DrawDebugType` "ForDuration"))
      (if _returnvalue_4
        (bind _returnvalue_5 (+ (`.Location` (`GameplayStatics.BreakHitResult` _outhit_2)) (0.0 0.0 30.0)))
        (bind _returnvalue_6 (+ _returnvalue_5 (* (`KismetMathLibrary.GetForwardVector` (`self.K2_GetActorRotation` _character_bp)) (75.0 75.0 0.0))))
        (bind (_outhit_3 _returnvalue_7) (`KismetSystemLibrary.LineTraceSingle` :`Start` _returnvalue_5 :`End` _returnvalue_6 :`TraceChannel` "TraceTypeQuery1" :`DrawDebugType` "ForDuration"))
        (`PrimitiveComponent.SetCollisionEnabled` (`self.Item mesh`) "QueryAndPhysics")
        (`self.K2_DetachFromActor` "KeepWorld" "KeepWorld" "KeepWorld")
        (if _returnvalue_7
          (`self.K2_SetActorTransform` (`KismetMathLibrary.MakeTransform` (`.Location` (`GameplayStatics.BreakHitResult` _outhit_3)) (struct :`Pitch` -90.0)))
          (else
            (`self.K2_SetActorTransform` (`KismetMathLibrary.MakeTransform` _returnvalue_6 (struct :`Pitch` -90.0)))))
        (bind _asfirst_person_anim_bp_2 (cast `/Game/FirstPersonArms/Animations/FirstPerson_AnimBP` (`SkeletalMeshComponent.GetAnimInstance` (`/Game/FirstPerson/Blueprints/BP_FirstPersonCharacter_New.FirstPersonMesh` (`self.Character BP`)))))
        (set `/Game/FirstPersonArms/Animations/FirstPerson_AnimBP.HasRifle` false _asfirst_person_anim_bp_2)))))

(event `self.Interact Item`
  ;[1 1 1] If you interact while looking at a locked door, it will consume the key
  (bind _outhit (`/Game/FirstPerson/Blueprints/BP_FirstPersonCharacter_New.Raycast` (`self.Character BP`)))
  (bind (_bblockinghit _binitialoverlap _time _distance _location _impactpoint _normal _impactnormal _physmat _hitactor) (`GameplayStatics.BreakHitResult` _outhit))
  (if (== _hitactor (`self.Door`))
    (message `/Game/BP/Interfaces/I_Unlock.Unlock` _hitactor)
    (`self.UseAndDeleteItem`)
    (`KismetSystemLibrary.PrintString` "unlocked! add sound here!")
    (else
      (bind _asbp_door (cast `/Game/BP/BP_Door` _hitactor)
        (:`then`
          (if (`/Game/BP/BP_Door.IsLocked` _asbp_door)
            (bind _returnvalue (`GameplayStatics.GetActorOfClass` "/Game/FirstPerson/Blueprints/BP_FirstPersonCharacter_New.BP_FirstPersonCharacter_New_C" :!label _label))
            (`/Game/Developers/JTLib/WBP_SUBTITLE.MakeSubtitle` (`/Game/FirstPerson/Blueprints/BP_FirstPersonCharacter_New.Subtitle Widget` _returnvalue) "Wrong Door" 0.1 1.0)))
        (:`CastFailed`
          (bind _asbp_double_door (cast `/Game/BP/BP_Double_Door` _hitactor))
          (if (`/Game/BP/BP_Double_Door.IsLocked` _asbp_double_door)
            (goto _label)))))))

(event `/Game/BP/Classes/InteractableBaseClass.Show Info`
  (params (HUD :type "/Game/BP/Widgets/WBP_HUD Object Reference"))
  ;[1 1 1] Comment
  (if (`/Game/FirstPerson/Blueprints/BP_FirstPersonCharacter_New.HasItem` (`self.Character BP`))
    (`/Game/BP/Widgets/WBP_HUD.Set Info Text` HUD "Can only hold one item")
    (else
      (`/Game/BP/Widgets/WBP_HUD.Set Info Text` HUD "Press [E] pick up"))))

(fn `UserConstructionScript`)