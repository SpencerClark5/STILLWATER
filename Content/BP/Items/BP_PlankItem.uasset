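; BP_PlankItem is a carried plank item that the player can drop on the ground or use up to fill a plank placement spot.
; DropItem traces downward from the character, then detaches the plank and moves it to just below the hit point, a fix marked temporary.
; InteractItem uses the character's raycast to find a non-deactivated BP_PlankObject, turns that plank on and deletes the held item, with a debug print standing in for sound.
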(event `self.DropItem`
  (bind _returnvalue (`self.K2_GetActorLocation` (`self.Character BP`)))
  (bind (_outhit _returnvalue_2) (`KismetSystemLibrary.LineTraceSingle` :`Start` _returnvalue :`End` (- _returnvalue (0.0 0.0 300.0)) :`TraceChannel` "TraceTypeQuery1" :`DrawDebugType` "Persistent"))
  (if _returnvalue_2
    (`self.K2_DetachFromActor` "KeepWorld" "KeepWorld" "KeepWorld")
    (`self.K2_SetActorTransform` (`KismetMathLibrary.MakeTransform` (+ (`.Location` (`GameplayStatics.BreakHitResult` _outhit)) (0.0 0.0 -5.0))))))

(event `self.Interact Item`
  ;[1 1 1] If you interact while looking at a unplaced plank, it will remove the plank from your hands and call interact on the place object
  (bind _outhit (`/Game/FirstPerson/Blueprints/BP_FirstPersonCharacter_New.Raycast` (`self.Character BP`)))
  (bind _asbp_plank_object (cast `/Game/BP/Objects/BP_PlankObject` (`.HitActor` (`GameplayStatics.BreakHitResult` _outhit))))
  (if (not (`/Game/BP/Objects/BP_PlankObject.Deactivated` _asbp_plank_object))
    (`/Game/BP/Objects/BP_PlankObject.Turn on plank` _asbp_plank_object)
    (`self.UseAndDeleteItem`)
    (`KismetSystemLibrary.PrintString` "placed! add sound here!")))

(fn `UserConstructionScript`)