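; BP_Key is a key item that the character holds and uses to unlock a locked BP_Door.
; Interacting uses the character's raycast, and if it hits a locked door, unlocks it and consumes the key.
; Dropping traces down from the character and, on a hit, detaches the key and places it above the ground with a temporary transform fix.
; ShowInfo sets the HUD pickup prompt, or a one-item limit message when the character already holds an item.
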(event `/Game/BP/Interfaces/I_Item.DropItem`
  (bind _returnvalue (`self.K2_GetActorLocation` (`self.Character BP`)))
  (bind (_outhit _returnvalue_2) (`KismetSystemLibrary.LineTraceSingle` :`Start` _returnvalue :`End` (- _returnvalue (0.0 0.0 300.0)) :`TraceChannel` "TraceTypeQuery1" :`DrawDebugType` "Persistent"))
  (if _returnvalue_2
    (`self.K2_DetachFromActor` "KeepWorld" "KeepWorld" "KeepWorld")
    (`self.K2_SetActorTransform` (`KismetMathLibrary.MakeTransform` (+ (`.Location` (`GameplayStatics.BreakHitResult` _outhit)) (0.0 0.0 30.0)) (struct :`Pitch` -90.0)))))

(event `/Game/BP/Interfaces/I_Item.Interact Item`
  ;[1 1 1] If you interact while looking at a locked door, it will consume the key
  (bind _outhit (`/Game/FirstPerson/Blueprints/BP_FirstPersonCharacter_New.Raycast` (`self.Character BP`)))
  (bind _asbp_door (cast `/Game/BP/Items/BP_Door` (`.HitActor` (`GameplayStatics.BreakHitResult` _outhit))))
  (if (`/Game/BP/Items/BP_Door.IsLocked` _asbp_door)
    (`/Game/BP/Items/BP_Door.Unlock door` _asbp_door)
    (`self.UseAndDeleteItem`)
    (`KismetSystemLibrary.PrintString` "unlocked! add sound here!")))

(event `/Game/BP/Interfaces/I_Interactable.Show Info`
  (params (HUD :type "/Game/BP/Widgets/WBP_HUD Object Reference"))
  (if (`/Game/FirstPerson/Blueprints/BP_FirstPersonCharacter_New.HasItem` (`self.Character BP`))
    (`/Game/BP/Widgets/WBP_HUD.Set Info Text` HUD "Can only hold one item")
    (else
      (`/Game/BP/Widgets/WBP_HUD.Set Info Text` HUD "Press [E] pick up"))))

(fn `UserConstructionScript`)