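; BP_RoamingMonster is a monster that wanders around its spawn point and chases pawns it sees.
; Roaming repeatedly moves it to random reachable points within a radius of its start position, pausing after each arrival.
; PawnSensing starts the chase, while a retriggerable delay returns it to roaming once sightings stop.
; Reaching the pawn destroys the monster and increments the CaughtByMonster count in BP_GameInstance, used for endings.
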(event `self.ReceiveBeginPlay`
  ;[0.5712 1 0.0828] Initialize variables and start random roaming
  (set `self.InitialPos` (`SceneComponent.K2_GetComponentLocation` (`self.CapsuleComponent`)))
  (`self.RandomRoaming` self))

(event `RandomRoaming`
  ;[1 0.8963 0.3419] Set random locations for AI to move to
  (`|AIMoveTo` self (`NavigationSystemV1.K2_GetRandomReachablePointInRadius` (`self.InitialPos`) 2000.0 null null) null
    (:`OnSuccess`
      (`KismetSystemLibrary.Delay` 1.0)
      (`self.RandomRoaming` self))))

(event `self.PawnSensing.OnSeePawn`
  (params (Pawn :type "Pawn Object Reference"))
  ;[1 0.8963 0.3419] Chase pawn seen
  (`|ExecutionSequence`
    (:`then_0`
      (`|AIMoveTo` self (0.0 0.0 0.0) Pawn
        (:`OnSuccess`
          (`KismetSystemLibrary.Delay` 0.3)
          (`self.K2_DestroyActor`)
          (bind _asbp_game_instance (cast `/Game/BP/BP_GameInstance` (`GameplayStatics.GetGameInstance`)))
          (bind _output_get (set `/Game/BP/BP_GameInstance.Caught by monster` (+ (`/Game/BP/BP_GameInstance.Caught by monster` _asbp_game_instance) 1) _asbp_game_instance)) ; Set global variable for endings
          (`KismetSystemLibrary.PrintString` (`KismetStringLibrary.Conv_IntToString` _output_get)))))
    (:`then_1`
      ;[0.2059 0.9403 1] Stop chasing when out of sight
      (`KismetSystemLibrary.RetriggerableDelay` 1.0)
      (`self.RandomRoaming`))))

(fn `UserConstructionScript`)