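; Drinkable water pickup that, when interacted with, temporarily reveals hidden actors through a "drank water" screen effect.
; BeginPlay caches the post-process volume tagged "Switch" and hides the BP_Key_Howie keys.
; Drinking adds M_DrankWater to that volume and shows I_Visible and I_KeyVisible actors with collision.
; After a timed delay it removes the material and re-hides only the I_Visible actors, leaving keys revealed.
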(event `self.ReceiveBeginPlay`
  ;[1 0.1958 0.9119] Set post process to variable in order to allow shader to be added later (during runtime)
  (bind _outactors (`GameplayStatics.GetAllActorsOfClassWithTag` "/Script/Engine.PostProcessVolume" "Switch"))
  (for _array_element _outactors
    (set `self.PostProcess` _array_element)
    (bind _outactors_2 (`GameplayStatics.GetAllActorsOfClass` "/Game/BP/Items/BP_Key_Howie.BP_Key_Howie_C"))
    (`self.SetActorHiddenInGame` _outactors_2 true)
    (`self.SetActorEnableCollision` _outactors_2 false)))

(event `/Game/BP/Interfaces/I_Object.Interact object`
  (bind _weightedblendable (make `WeightedBlendable` 1.0 "/Game/Materials/Shaders/M_DrankWater.M_DrankWater"))
  (bind _array (break `WeightedBlendables` (`.WeightedBlendables` (break `PostProcessSettings` (`PostProcessVolume.Settings` (`self.PostProcess`))))))
  ;[1 0.08653 0.7857] Add shader to post-processing volume when water is drank
  (`KismetSystemLibrary.Delay` 0.2)
  (`KismetArrayLibrary.Array_Add` _array _weightedblendable)
  (set `self.WaterIsDrank` true)
  (bind _outactors (`GameplayStatics.GetAllActorsWithInterface` "/Game/BP/Interfaces/I_Visible.I_Visible_C"))
  (for _array_element _outactors
    (message `/Game/BP/Interfaces/I_Visible.Toggle Visibility` _array_element)
    (`self.SetActorHiddenInGame` _array_element false)
    (`self.SetActorEnableCollision` _array_element true)
    (bind _outactors_2 (`GameplayStatics.GetAllActorsWithInterface` "/Game/BP/Interfaces/I_KeyVisible.I_KeyVisible_C"))
    (for _array_element_2 _outactors_2
      (`self.SetActorHiddenInGame` _array_element_2 false)
      (`self.SetActorEnableCollision` _array_element_2 true)
      (`KismetSystemLibrary.Delay` 15.0)
      (`KismetArrayLibrary.Array_RemoveItem` _array _weightedblendable)
      (set `self.WaterIsDrank` false)
      (for _array_element_3 _outactors
        (`self.SetActorHiddenInGame` _array_element_3 true)
        (`self.SetActorEnableCollision` _array_element_3 false)))))

(event `/Game/BP/Interfaces/I_Interactable.Show Info`
  (params (HUD :type "/Game/BP/Widgets/WBP_HUD Object Reference"))
  ;[0.2033 0.6384 1] Display text for water
  (`/Game/BP/Widgets/WBP_HUD.Set Info Text` HUD "Press [E] to drink"))

(fn `UserConstructionScript`)