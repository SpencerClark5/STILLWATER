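; BP_Car is the interactable escape car that ends the game once the player has unlocked it.
; An editor-set Status enum initializes the lock flag at BeginPlay and selects the HUD prompt in ShowInfo, either to find the key or to leave.
; Unlock switches the car to Close, letting InteractObject play a level sequence, wait for its playback length, then show the credits widget.
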(event `self.ReceiveBeginPlay`
  ;[1 1 1] Grabs whatever the editor has set to and sets status
  (switch `/Game/Enums/EN_DoorStatus` (`self.Status`)
    (:`NewEnumerator2`
      (set `self.IsLocked` true))
    (:`NewEnumerator0`
      (set `self.IsLocked` false :!label _label))
    (:`NewEnumerator1`
      (goto _label)))
  (bind _returnvalue (`GameplayStatics.GetActorOfClass` "/Game/FirstPerson/Blueprints/BP_FirstPersonCharacter_New.BP_FirstPersonCharacter_New_C"))
  (set `self.Character BP` _returnvalue))

(event `self.Interact object`
  (bind _movie (`self.Movie`))
  (if (not (`self.IsLocked`))
    (switch `/Game/Enums/EN_DoorStatus` (`self.Status`)
      (:`NewEnumerator0`
        (bind _outactor (`LevelSequencePlayer.CreateLevelSequencePlayer` _movie))
        (`MovieSceneSequencePlayer.Play` (`LevelSequenceActor.SequencePlayer` _outactor))
        (bind _returnvalue (`MovieSceneSequenceExtensions.GetPlaybackEndSeconds` _movie))
        (`KismetSystemLibrary.Delay` _returnvalue)
        (bind _returnvalue_2 (`|CreateWidget` "/Game/BP/Widgets/WBP_Credits.WBP_Credits_C"))
        (`UserWidget.AddToViewport` _returnvalue_2 0)))))

(event `/Game/BP/Classes/InteractableBaseClass.Show Info`
  (params (HUD :type "/Game/BP/Widgets/WBP_HUD Object Reference"))
  ;[1 1 1] When the players normal looking raycast hits the door, display some text on the widget
  (switch `/Game/Enums/EN_DoorStatus` (`self.Status`)
    (:`NewEnumerator2`
      (`/Game/BP/Widgets/WBP_HUD.Set Info Text` HUD "Find the car key")
      (set `TextBlock.Text` "Use LMB to unlock door" (`/Game/BP/Widgets/WBP_HUD.InteractInfo` HUD)))
    (:`NewEnumerator0`
      (`/Game/BP/Widgets/WBP_HUD.Set Info Text` HUD "Press [E] to Leave"))
    (:`NewEnumerator1`
      (`/Game/BP/Widgets/WBP_HUD.Set Info Text` HUD "Wrong State"))))

(event `self.Unlock`
  (set `self.Status` "NewEnumerator0")
  (set `self.IsLocked` false))

(fn `UserConstructionScript`)